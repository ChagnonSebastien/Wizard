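; Playing card actor that animates itself through dealing, hand layout and flipping, and shows its value and suit through a dynamic material.
; Looping timers step clamped moves: Distribute flies the card to a player's arm point, attaches it, then hands off to layout updates.
; Layout fans cards by position and hand size, spreading around and scaling the hovered card, and raises and centers one prepared for drop.
; Flip turns it along a sine arc.
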(event `Cancel Held`
  (`KismetSystemLibrary.K2_ClearAndInvalidateTimerHandle` (`self.Movement Handle`))
  (`KismetSystemLibrary.K2_ClearAndInvalidateTimerHandle` (`self.Distribute Handle`)))

(event `Update Prepare Drop`
  (params (`Drop Prepared` :type Boolean))
  (bind _position (`self.Position`))
  (bind _hover (`self.Hover`))
  (bind _returnvalue (>= _hover 0))
  (bind _relativelocation (`SceneComponent.RelativeLocation` (`self.Arm`)))
  (bind _yaw (.yaw (`SceneComponent.RelativeRotation` (`self.Arm`))))
  (bind _x (.x (`SceneComponent.RelativeScale3D` (`self.Card Component`))))
  (bind _returnvalue_2 (`KismetMathLibrary.Conv_IntToDouble` (- (`self.Hand Size`) 1)))
  (bind _returnvalue_3 (- (`KismetMathLibrary.MakeVector` 0.0 0.0 (`KismetMathLibrary.SelectFloat` 15.0 0.0 (`self.Prepared Drop`))) _relativelocation))
  (bind _returnvalue_4 (- (`KismetMathLibrary.SelectFloat` 1.0 0.75 (== (`self.Position`) (`self.Hover`))) _x))
  (bind _returnvalue_5 (* -12 (`KismetMathLibrary.Sqrt` _returnvalue_2)))
  (bind _returnvalue_6 (`KismetMathLibrary.VSize` _returnvalue_3))
  (bind _returnvalue_7 (> (`KismetMathLibrary.Abs` _returnvalue_4) 0.001))
  (bind _returnvalue_8 (/ 20.0 (+ (* 1 (.z _relativelocation)) 1.0)))
  (bind _returnvalue_9 (<= _returnvalue_6 0.001))
  (bind _returnvalue_10 (+ _x (`KismetMathLibrary.FClamp` _returnvalue_4 -0.1 0.1)))
  (bind _returnvalue_11 (- (`KismetMathLibrary.SelectFloat` 0.0 (+ (/ _returnvalue_5 -2.0) (* (`self.Position`) (/ _returnvalue_5 _returnvalue_2)) (`KismetMathLibrary.SelectFloat` -3.0 0.0 (and (> _position _hover) _returnvalue)) (`KismetMathLibrary.SelectFloat` 3.0 0.0 (and _returnvalue (< _position _hover)))) (`self.Prepared Drop`)) _yaw))
  (bind _returnvalue_12 (<= (`KismetMathLibrary.Abs` _returnvalue_11) 0.001))
  (set `self.Prepared Drop` `Drop Prepared`)
  (if (not (`KismetSystemLibrary.K2_IsTimerActiveHandle` (`self.Distribute Handle`))) :!label _label
    (`KismetSystemLibrary.K2_ClearAndInvalidateTimerHandle` (`self.Movement Handle`))
    (bind _returnvalue_13 (`KismetSystemLibrary.K2_SetTimerDelegate` (delegate `Recalculate Position`) 0.041667 true))
    (set `self.Movement Handle` _returnvalue_13)
    (if _returnvalue_7 :!label _label_2
      (`SceneComponent.SetRelativeScale3D` (`self.Card Component`) (`KismetMathLibrary.MakeVector` _returnvalue_10 _returnvalue_10 _returnvalue_10)))
    (if _returnvalue_9
      _
      (else
        _))
    (`SceneComponent.K2_SetRelativeLocation` (`self.Arm`) (+ (* (`KismetMathLibrary.Normal` _returnvalue_3 0.0) (`KismetMathLibrary.FClamp` _returnvalue_6 (* -1 _returnvalue_8) _returnvalue_8)) _relativelocation) false false)
    (if (not _returnvalue_12)
      (`SceneComponent.K2_SetRelativeRotation` (`self.Arm`) (`KismetMathLibrary.MakeRotator` (.roll (`SceneComponent.RelativeRotation` (`self.Arm`))) (.pitch (`SceneComponent.RelativeRotation` (`self.Arm`))) (+ _yaw (`KismetMathLibrary.FClamp` _returnvalue_11 -5.0 5.0))) false false))
    (if (and _returnvalue_12 (not _returnvalue_7) _returnvalue_9)
      (`KismetSystemLibrary.K2_ClearAndInvalidateTimerHandle` (`self.Movement Handle`)))))

(event `Update Swap`
  (params (Position :type Integer) (Hover :type Integer))
  (set `self.Position` Position)
  (set `self.Hover` Hover)
  (goto _label))

(event `Recalculate Position`
  (goto _label_2))

(event `Update Hover`
  (params (Hover :type Integer))
  (set `self.Hover` Hover)
  (goto _label))

(event `Update Position`
  (params (Position :type Integer) (`Hand Size` :type Integer))
  (set `self.Position` Position)
  (set `self.Hand Size` `Hand Size`)
  (set `self.Hover` -1)
  (goto _label))

(event `Distribute`
  (params (Arm :type "SceneComponent Object Reference") (Position :type Integer) (`Hand Size` :type Integer))
  (bind _defaultsceneroot (`self.DefaultSceneRoot`))
  (bind _location (.location (`SceneComponent.K2_GetComponentToWorld` (`self.DefaultSceneRoot`))))
  (bind _roll (.roll (`SceneComponent.RelativeRotation` (`self.Card Component`))))
  (bind _yaw (.yaw (.rotation (`SceneComponent.K2_GetComponentToWorld` (`self.DefaultSceneRoot`)))))
  (bind _returnvalue (- -120.0 _roll))
  (bind _returnvalue_2 (- (+ (.z (`SceneComponent.K2_GetComponentLocation` (`self.Player Point Reference`))) 0.0) (.z (`SceneComponent.K2_GetComponentLocation` (`self.DefaultSceneRoot`)))))
  (bind _returnvalue_3 (- (+ (.location (`SceneComponent.K2_GetComponentToWorld` (`self.Player Point Reference`))) (0.0 0.0 0.0)) _location))
  (bind _returnvalue_4 (<= -0.001 _returnvalue))
  (bind _returnvalue_5 (- (`KismetMathLibrary.VSize` _returnvalue_3) 55.0))
  (bind _returnvalue_6 (- (- (mod (+ (.yaw (.rotation (`SceneComponent.K2_GetComponentToWorld` (`self.Player Point Reference`)))) 270.0 360.0) 360.0) 179.999893) _yaw))
  (bind _returnvalue_7 (and (<= _returnvalue_5 0.001) (<= (`KismetMathLibrary.Abs` _returnvalue_6) 0.001)))
  (set `self.Position` Position)
  (set `self.Hand Size` `Hand Size`)
  (set `self.Player Point Reference` Arm)
  (bind _returnvalue_8 (`KismetSystemLibrary.K2_SetTimerDelegate` (delegate `Distribution Step`) 0.041667 true))
  (set `self.Distribute Handle` _returnvalue_8)
  (if (== _returnvalue_2 0.0) :!label _label_3
    (if (not _returnvalue_7)
      (`SceneComponent.K2_SetWorldTransform` (`self.DefaultSceneRoot`) (`KismetMathLibrary.MakeTransform` (+ (* (`KismetMathLibrary.Normal` _returnvalue_3 0.0) (`KismetMathLibrary.FClamp` _returnvalue_5 -12.5 12.5)) _location) (`KismetMathLibrary.MakeRotator` (.roll (.rotation (`SceneComponent.K2_GetComponentToWorld` (`self.DefaultSceneRoot`)))) (.pitch (.rotation (`SceneComponent.K2_GetComponentToWorld` (`self.DefaultSceneRoot`)))) (+ (`KismetMathLibrary.FClamp` _returnvalue_6 -17.5 17.5) _yaw)) (.scale (`SceneComponent.K2_GetComponentToWorld` (`self.DefaultSceneRoot`)))) false false))
    (if (not _returnvalue_4)
      (`SceneComponent.K2_SetRelativeRotation` (`self.Card Component`) (`KismetMathLibrary.MakeRotator` (+ _roll (`KismetMathLibrary.FClamp` _returnvalue -20.0 20.0)) 0.0 8.0) false false))
    (if (and _returnvalue_7 _returnvalue_4)
      (`SceneComponent.K2_SetWorldTransform` (`self.RotationPoint`) (`SceneComponent.K2_GetComponentToWorld` (`self.Player Point Reference`)) false false)
      (`SceneComponent.K2_AttachToComponent` (`self.Hand`) (`self.Arm`) "None" "KeepWorld" "KeepWorld" "KeepWorld" false)
      (`KismetSystemLibrary.K2_ClearAndInvalidateTimerHandle` (`self.Distribute Handle`))
      (`self.Update Position` (`self.Position`) (`self.Hand Size`)))
    (else
      (`SceneComponent.K2_SetRelativeLocation` _defaultsceneroot (+ (`SceneComponent.RelativeLocation` _defaultsceneroot) (`KismetMathLibrary.MakeVector` 0.0 0.0 (`KismetMathLibrary.FClamp` _returnvalue_2 -1.5 1.5))) false false))))

(event `Distribution Step`
  (goto _label_3))

(event `Flip`
  (set `self.Revealed` true)
  (bind _returnvalue (`KismetSystemLibrary.K2_SetTimerDelegate` (delegate `Turn Step`) 0.041667 true)))

(event `Turn Step`
  (bind _hand (`self.Hand`))
  (bind _output_get (set `self.Turn Offset` (`KismetMathLibrary.FMin` (+ (`self.Turn Offset`) 0.08) 1.0)))
  (if (== _output_get 1.0)
    (`KismetSystemLibrary.K2_ClearAndInvalidateTimerHandle` (stale `Flip` _returnvalue)))
  (`SceneComponent.K2_SetRelativeRotation` _hand (`KismetMathLibrary.MakeRotator` 0.0 (* -180 _output_get)) false false)
  (`SceneComponent.K2_SetRelativeLocation` _hand (`KismetMathLibrary.MakeVector` 0.0 0.0 (* -15 (`KismetMathLibrary.Sin` (`KismetMathLibrary.MultiplyByPi` _output_get)))) false false))

(fn `CreateDynamicMarerial`
  (bind _returnvalue (`PrimitiveComponent.CreateDynamicMaterialInstance` (`self.Card`) 2 "/Game/Assets/Card/CardFront_Material.CardFront_Material" "None"))
  (set `self.Material` _returnvalue))

(fn `Set Content`
  (params (Content :type "/Game/Blueprints/Card/CardContent Structure"))
  (locals (`Card Face` :type "Float (double-precision)"))
  (bind _output_get (set `self.CardContent` Content))
  (`/Engine/EditorBlueprintResources/StandardMacros.IsValid` (`self.Material`)
    (:`Is Valid`
      _)
    (:`Is Not Valid`
      (`self.CreateDynamicMarerial`)))
  (`|ExecutionSequence`
    (:`then_0`
      (bind (_type _value) (break `/Game/Blueprints/Card/CardContent` _output_get))
      (switch `/Game/Blueprints/Card/CardValue` _value
        (:`NewEnumerator1`
          (set `local.Card Face` 1.0))
        (:`NewEnumerator2`
          (set `local.Card Face` 2.0))
        (:`NewEnumerator3`
          (set `local.Card Face` 3.0))
        (:`NewEnumerator4`
          (set `local.Card Face` 4.0))
        (:`NewEnumerator5`
          (set `local.Card Face` 5.0))
        (:`NewEnumerator6`
          (set `local.Card Face` 6.0))
        (:`NewEnumerator7`
          (set `local.Card Face` 7.0))
        (:`NewEnumerator8`
          (set `local.Card Face` 8.0))
        (:`NewEnumerator9`
          (set `local.Card Face` 9.0))
        (:`NewEnumerator10`
          (set `local.Card Face` 10.0))
        (:`NewEnumerator11`
          (set `local.Card Face` 11.0))
        (:`NewEnumerator12`
          (set `local.Card Face` 12.0))
        (:`NewEnumerator0`
          (set `local.Card Face` 0.0))
        (:`NewEnumerator13`
          (set `local.Card Face` 13.0))
        (:`NewEnumerator14`
          (set `local.Card Face` 14.0))))
    (:`then_1`
      (`MaterialInstanceDynamic.SetScalarParameterValue` (`self.Material`) "Card Number" (`local.Card Face`))
      (`MaterialInstanceDynamic.SetScalarParameterValue` (`self.Material`) "Card Sign" (`KismetMathLibrary.Conv_ByteToDouble` _type)))))

(fn `UserConstructionScript`)