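; Card deck actor that spawns and holds 60 face-flipped cards and tracks those moved to the table.
; BeginPlay stacks the cards upward as attached actors, filling the array in reverse so index 0 is the top card.
; Next returns the card at a running Offset, while PutOnTable moves a given card from Cards to Table.
; CleanTable destroys the table's cards, and destroying the deck destroys both sets.
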(event `self.ReceiveBeginPlay`
  (for _index (range 60)
    (bind _returnvalue (`|SpawnActorFromClass` "/Game/Blueprints/Card/Card.Card_C" (`KismetMathLibrary.MakeTransform` (`KismetMathLibrary.MakeVector` 0.0 0.0 (* _index 0.075)) (struct :`Roll` 180.0)) "AlwaysSpawn" "OverrideRootScale" null null))
    (`KismetArrayLibrary.Array_Set` (`self.Cards`) (- 59 _index) _returnvalue true)
    (`self.K2_AttachToComponent` _returnvalue (`self.DefaultSceneRoot`) "None" "KeepRelative" "KeepRelative" "KeepRelative" false)))

(event `self.ReceiveDestroyed`
  (for _array_element (`self.Cards`)
    (`self.K2_DestroyActor` _array_element))
  (`self.Clean Table`))

(event `Put On Table`
  (params (Card :type "/Game/Blueprints/Card/Card Object Reference"))
  (`KismetArrayLibrary.Array_Add` (`self.Table`) Card)
  (`KismetArrayLibrary.Array_RemoveItem` (`self.Cards`) Card))

(event `Clean Table`
  (bind _table (`self.Table`))
  (for _array_element _table
    (`self.K2_DestroyActor` _array_element))
  (`KismetArrayLibrary.Array_Clear` _table))

(fn `Next`
  (returns (Next :type "/Game/Blueprints/Card/Card Object Reference"))
  (locals (Card :type "/Game/Blueprints/Card/Card Object Reference"))
  (bind _offset (`self.Offset`))
  (bind _output_get (set `local.Card` (`|GetArrayItem` (`self.Cards`) _offset)))
  (`/Engine/EditorBlueprintResources/StandardMacros.IncrementInt` _offset
    (:`  `
      (return _output_get))))

(fn `UserConstructionScript`)