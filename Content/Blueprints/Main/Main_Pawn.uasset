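; Player pawn for a networked trump-and-prediction card game, holding the player's hand and forwarding trump choices, predictions and plays to Main_GameState.
; Dealt cards are tracked by ID in maps for actors and contents, plus an array for display order.
; For the owner, Tick traces the cursor to hover cards, reorder dragged ones by angle, or raise them in the upper screen half.
; Releasing there on turn plays the card; DropCard tosses it tableward with physics.
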(event `Send Trump Selection`
  (params (`Trump Selection` :type "/Game/Blueprints/Card/CardType Enum" :default "NewEnumerator0"))
  (bind _asmain_game_state (cast `/Game/Blueprints/Main/Main_GameState` (`GameplayStatics.GetGameState`)))
  (`/Game/Blueprints/Main/Main_GameState.Select Trump` _asmain_game_state self `Trump Selection`))

(event `Send Prediction`
  (params (Prediction :type Integer))
  (bind _asmain_game_state (cast `/Game/Blueprints/Main/Main_GameState` (`GameplayStatics.GetGameState`)))
  (`/Game/Blueprints/Main/Main_GameState.Make Prediction` _asmain_game_state self Prediction))

(event `Turn Change Handler`
  (params (OwnTurn :type Boolean))
  (set `self.Own Turn` OwnTurn))

(event `New Deck Spawned Handler`
  (params (Deck :type "/Game/Blueprints/Card/Deck Object Reference"))
  (set `self.Deck Reference` Deck)
  (`BlueprintMapLibrary.Map_Clear` (`self.Hand`))
  (`BlueprintMapLibrary.Map_Clear` (`self.HandContent`))
  (`KismetArrayLibrary.Array_Clear` (`self.Card Order`)))

(event `Play Card`
  (params (`Card ID` :type Integer))
  (bind _asmain_game_state (cast `/Game/Blueprints/Main/Main_GameState` (`GameplayStatics.GetGameState`)))
  (`/Game/Blueprints/Main/Main_GameState.PlayCard` _asmain_game_state self `Card ID`))

(event `Left Click`
  (bind _last_index (`self.Last Index`))
  (if (>= _last_index 0)
    (set `self.Moving Card` (`BlueprintMapLibrary.Map_Find` (`self.Hand`) (`|GetArrayItem` (`self.Card Order`) _last_index)))))

(event `Distribute`
  (params (`Card ID` :type Integer) (Content :type "/Game/Blueprints/Card/CardContent Structure"))
  (`/Engine/EditorBlueprintResources/ActorMacros.Switch Has Authority`
    (:`Authority`
      (`self.TakeCard` `Card ID`)
      (`self.IdentifyCard` `Card ID` Content))))

(event `TakeCard`
  (params (`Card ID` :type Integer))
  (bind _card_order (`self.Card Order`))
  (bind _returnvalue (`KismetArrayLibrary.Array_Length` _card_order))
  (bind (_value _returnvalue_2) (`BlueprintMapLibrary.Map_Find` (`self.HandContent`) `Card ID`))
  (bind _asmain_game_state (cast `/Game/Blueprints/Main/Main_GameState` (`GameplayStatics.GetGameState`)))
  (bind _next (`/Game/Blueprints/Card/Deck.Next` (`/Game/Blueprints/Main/Main_GameState.Deck` _asmain_game_state)))
  (`BlueprintMapLibrary.Map_Add` (`self.Hand`) `Card ID` _next)
  (if _returnvalue_2
    (`/Game/Blueprints/Card/Card.Set Content` _next _value))
  (for (_array_element _array_index) _card_order
    (`/Game/Blueprints/Card/Card.Update Position` (`BlueprintMapLibrary.Map_Find` (`self.Hand`) _array_element) _array_index (+ _returnvalue 1)))
  (bind _returnvalue_3 (`KismetArrayLibrary.Array_Add` _card_order _returnvalue))
  (`/Game/Blueprints/Card/Card.Distribute` _next (`self.Card Anchor`) _returnvalue_3 _returnvalue))

(event `Left Release`
  (`/Engine/EditorBlueprintResources/StandardMacros.IsValid` (`self.Moving Card`)
    (:`Is Valid`
      (if (and (`self.Own Turn`) (`self.Prepared Drop`))
        (`self.Play Card` (`|GetArrayItem` (`self.Card Order`) (`self.Last Index`)))
        (set `self.Moving Card` null)
        (else
          (set `self.Moving Card` null)
          (`self.Cancel Drop` (`|GetArrayItem` (`self.Card Order`) (`self.Last Index`)))
          (set `self.Prepared Drop` false))))))

(event `IdentifyCard`
  (params (`Card ID` :type Integer) (Content :type "/Game/Blueprints/Card/CardContent Structure"))
  (bind (_value _returnvalue) (`BlueprintMapLibrary.Map_Find` (`self.Hand`) `Card ID`))
  (`BlueprintMapLibrary.Map_Add` (`self.HandContent`) `Card ID` Content)
  (if _returnvalue
    (`/Game/Blueprints/Card/Card.Set Content` _value Content)))

(event `Drop Card`
  (params (`Card ID` :type Integer) (`Card Content` :type "/Game/Blueprints/Card/CardContent Structure"))
  (bind _card_order (`self.Card Order`))
  (bind _value (`BlueprintMapLibrary.Map_Find` (`self.Hand`) `Card ID`))
  (bind _card (`/Game/Blueprints/Card/Card.Card` _value))
  (set `self.Own Turn` false)
  (set `self.Moving Card` null)
  (set `self.Last Index` -1)
  (`/Game/Blueprints/Card/Card.Set Content` _value `Card Content`)
  (`/Game/Blueprints/Card/Card.Cancel Held` _value)
  (`|ExecutionSequence`
    (:`then_0`
      (`/Game/Blueprints/Card/Deck.Put On Table` (`/Game/Blueprints/Main/Main_GameState.Deck` (cast `/Game/Blueprints/Main/Main_GameState` (`GameplayStatics.GetGameState`) :!pure true)) _value)
      (`PrimitiveComponent.SetSimulatePhysics` _card true)
      (`SceneComponent.K2_SetWorldLocation` _card (`KismetMathLibrary.MakeVector` (.x (`SceneComponent.K2_GetComponentLocation` _card)) (.y (`SceneComponent.K2_GetComponentLocation` _card)) 90.0) false false)
      (`PrimitiveComponent.SetAllPhysicsLinearVelocity` _card (* (`KismetMathLibrary.MakeVector` (.x (`SceneComponent.K2_GetComponentLocation` _card)) (.y (`SceneComponent.K2_GetComponentLocation` _card))) -2) false)
      (set `/Game/Blueprints/Card/Card.Revealed` true _value))
    (:`then_1`
      (`BlueprintMapLibrary.Map_Remove` (`self.Hand`) `Card ID`)
      (`KismetArrayLibrary.Array_Remove` _card_order (`self.Get Card Index from ID` `Card ID`))
      (for (_array_element _array_index) _card_order
        (`/Game/Blueprints/Card/Card.Update Position` (`BlueprintMapLibrary.Map_Find` (`self.Hand`) _array_element) _array_index (`KismetArrayLibrary.Array_Length` (`self.Card Order`)))))))

(event `self.ReceiveTick`
  (params (DeltaSeconds :type "Float (single-precision)"))
  (bind (_bblockinghit _binitialoverlap _time _distance _location _impactpoint _normal _impactnormal _physmat _hitactor) (`GameplayStatics.BreakHitResult` (`PlayerController.GetHitResultUnderCursorByChannel` (`GameplayStatics.GetPlayerController` 0) "TraceTypeQuery2" true)))
  (if (`self.Is Owner`)
    (`/Engine/EditorBlueprintResources/StandardMacros.IsValid` (`self.Moving Card`)
      (:`Is Valid`
        (`self.Card Follow Mouse`))
      (:`Is Not Valid`
        (`/Engine/EditorBlueprintResources/StandardMacros.IsValid` _hitactor
          (:`Is Valid`
            (bind _ascard (cast `/Game/Blueprints/Card/Card` _hitactor)
              (:`then`
                (bind _values (`BlueprintMapLibrary.Map_Values` (`self.Hand`)))
                (if (`KismetArrayLibrary.Array_Contains` _values _ascard)
                  (bind _index (`self.Get Card Index from ID` (`self.Get Card ID from Actor` _ascard)))
                  (if (!= _index (`self.Last Index`))
                    (bind _output_get (set `self.Last Index` _index))
                    (`self.Start Hover` _output_get))))
              (:`CastFailed`
                (if (>= (`self.Last Index`) 0) :!label _label
                  (set `self.Last Index` -1)
                  (`self.Stop Hover`)))))
          (:`Is Not Valid`
            (goto _label)))))))

(event `Start Hover`
  (params (Index :type Integer))
  (`self.Set Hover` Index))

(event `Stop Hover`
  (`self.Set Hover` -1))

(event `Set Hover`
  (params (Index :type Integer))
  (bind _values (`BlueprintMapLibrary.Map_Values` (`self.Hand`)))
  (for _array_element _values
    (`/Game/Blueprints/Card/Card.Update Hover` _array_element Index)))

(event `Card Follow Mouse`
  (bind _returnvalue (`GameplayStatics.GetPlayerController` 0))
  (bind _moving_card (`self.Moving Card`))
  (bind _prepared_drop (`self.Prepared Drop`))
  (bind (_worldlocation _worlddirection) (`PlayerController.DeprojectMousePositionToWorld` _returnvalue))
  (bind _worldlocation_2 (`PlayerController.DeprojectMousePositionToWorld` (`GameplayStatics.GetPlayerController` 0)))
  (bind _output (`|GetArrayItem` (`self.Card Order`) (`self.Last Index`)))
  (bind _returnvalue_2 (`KismetMathLibrary.MakeVector` (.x _worldlocation) (.y _worldlocation) (+ (.z (`SceneComponent.K2_GetComponentLocation` (`self.Card Anchor`))) 5.0)))
  (if (< (/ (`.LocationY` (`PlayerController.GetMousePosition` _returnvalue)) (`KismetMathLibrary.Conv_IntToDouble` (`.SizeY` (`PlayerController.GetViewportSize` _returnvalue)))) 0.5)
    (if (not _prepared_drop)
      (`self.Prepare Drop` _output)
      (set `self.Prepared Drop` true))
    (else
      (if _prepared_drop
        (`self.Cancel Drop` _output)
        (set `self.Prepared Drop` false))
      (bind _outhit (`KismetSystemLibrary.LineTraceSingle` _returnvalue_2 (+ _returnvalue_2 (* (`KismetMathLibrary.MakeVector` (.x _worlddirection) (.y _worlddirection)) 100)) "TraceTypeQuery2"))
      (bind _ascard (cast `/Game/Blueprints/Card/Card` (`.HitActor` (`GameplayStatics.BreakHitResult` _outhit))))
      (if (== _ascard _moving_card)
        _
        (elif (< (`self.Angle 2D` (- (`SceneComponent.K2_GetComponentLocation` (`/Game/Blueprints/Card/Card.Card` _ascard)) _worldlocation_2) (- (`SceneComponent.K2_GetComponentLocation` (`/Game/Blueprints/Card/Card.Card` _moving_card)) _worldlocation_2)) 0.0)
          (bind _index (`self.Get Card Index from ID` (`self.Get Card ID from Actor` _ascard)))
          (if (> _index (`self.Last Index`))
            (bind _output_get (set `self.Previous Last Index` (`self.Last Index`) :!label _label_2))
            (set `self.Last Index` (+ (- _index _output_get) _output_get))
            (`self.Swap Cards` _output_get _index))
          (elif (< _index (`self.Last Index`))
            (goto _label_2)))))))

(event `Swap Cards`
  (params (Active :type Integer) (`Swap With` :type Integer))
  (`self.Exchange Cards` Active `Swap With`))

(event `Exchange Cards`
  (params (Active :type Integer) (`Swap With` :type Integer))
  (bind _card_order (`self.Card Order`))
  (bind (_index _previous) (`self.From To Loop With Break` Active `Swap With` true)
    (:`Body`
      (`KismetArrayLibrary.Array_Swap` _card_order _index _previous)
      (`/Game/Blueprints/Card/Card.Update Swap` (`BlueprintMapLibrary.Map_Find` (`self.Hand`) (`|GetArrayItem` _card_order _previous)) _previous `Swap With`))
    (:`Finished`
      (`/Game/Blueprints/Card/Card.Update Swap` (`BlueprintMapLibrary.Map_Find` (`self.Hand`) (`|GetArrayItem` _card_order `Swap With`)) `Swap With` `Swap With`))))

(event `Prepare Drop`
  (params (`Card ID` :type Integer))
  (`self.Raise Card` `Card ID`))

(event `Raise Card`
  (params (`Card ID` :type Integer))
  (bind (_value _returnvalue) (`BlueprintMapLibrary.Map_Find` (`self.Hand`) `Card ID`))
  (if _returnvalue
    (`/Game/Blueprints/Card/Card.Update Prepare Drop` _value true)))

(event `Cancel Drop`
  (params (`Card ID` :type Integer))
  (`self.Lower Card` `Card ID`))

(event `Lower Card`
  (params (`Card ID` :type Integer))
  (bind (_value _returnvalue) (`BlueprintMapLibrary.Map_Find` (`self.Hand`) `Card ID`))
  (if _returnvalue
    (`/Game/Blueprints/Card/Card.Update Prepare Drop` _value false)))

(fn `Angle 2D`
  (params (V1 :type "Vector Structure") (V2 :type "Vector Structure"))
  (returns (Angle :type "Float (double-precision)"))
  (return (- (`KismetMathLibrary.DegAtan2` (.y V1) (.x V1)) (`KismetMathLibrary.DegAtan2` (.y V2) (.x V2)))))

(fn `Get Card ID from Actor`
  (params (Card :type "/Game/Blueprints/Card/Card Object Reference"))
  (returns (ID :type Integer))
  (locals (Key :type Integer))
  (bind _hand (`self.Hand`))
  (bind _keys (`BlueprintMapLibrary.Map_Keys` _hand))
  (for _array_element _keys
    (if (== Card (`BlueprintMapLibrary.Map_Find` _hand _array_element))
      (set `local.Key` _array_element)
      (break)))
  (return (`local.Key`)))

(fn `Get Card Index from ID`
  (params (`Card ID` :type Integer))
  (returns (Index :type Integer))
  (return (`KismetArrayLibrary.Array_Find` (`self.Card Order`) `Card ID`)))

(fn `Is Owner`
  (returns (Owner :type Boolean))
  (return (== (`self.GetController`) (`GameplayStatics.GetPlayerController` 0))))

(fn `Is Scoreboard Open`
  (returns (`Should Be Open` :type Boolean))
  (bind _returnvalue (`GameplayStatics.GetPlayerController` 0))
  (bind (_locationx _locationy) (`PlayerController.GetMousePosition` _returnvalue))
  (return (and (< (- (`PlayerController.GetViewportSize` _returnvalue) (`KismetMathLibrary.FTrunc` _locationx)) 100) (< _locationy 50.0))))

(fn `OnRep_HatMesh`
  (`StaticMeshComponent.SetStaticMesh` (`self.Hat`) (`self.HatMesh`)))

(fn `UserConstructionScript`)