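; Game mode for a multiplayer wizard table game that gathers joining player controllers and starts the match once the lobby reaches the game instance's max player count.
; Respawning names the pawn and respaces all players evenly in a circle facing the table using sine and cosine.
; After a short timer, it hands the controllers to the game state and has each one identify the other players' pawns.
; Logout asks the game instance to destroy that player's session.
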(event `self.ReceiveBeginPlay`
  ;[1 1 1] If the host, gets the amount of players and verifies the starting condition
  (`/Engine/EditorBlueprintResources/ActorMacros.Switch Has Authority`
    (:`Authority`
      (bind _aswizard_game_instance (cast `/Game/Blueprints/WizardGameInstance` (`GameplayStatics.GetGameInstance`)))
      (set `self.Max Players` (`/Game/Blueprints/WizardGameInstance.MaxPlayers` _aswizard_game_instance))
      (`self.CheckStartingContition`))))

(event `self.K2_PostLogin`
  (params (NewPlayer :type "PlayerController Object Reference"))
  ;[1 1 1] New Player Joins the map - Gets the player Controller and checks the starting condition
  (bind _asmain_player_controller (cast `/Game/Blueprints/Main/Main_PlayerController` NewPlayer))
  (`KismetArrayLibrary.Array_Add` (`self.PlayerControllers`) _asmain_player_controller)
  (`self.CheckStartingContition` :!label _label))

(event `self.K2_OnSwapPlayerControllers`
  (params (OldPC :type "PlayerController Object Reference") (NewPC :type "PlayerController Object Reference"))
  ;[1 1 1] New Player Joins the map - Gets the player Controller and checks the starting condition
  (bind _asmain_player_controller (cast `/Game/Blueprints/Main/Main_PlayerController` NewPC))
  (`KismetArrayLibrary.Array_Add` (`self.PlayerControllers`) _asmain_player_controller)
  (goto _label))

(event `RespawnPlayer`
  (params (Player :type "/Game/Blueprints/Main/Main_PlayerController Object Reference") (Name :type Text))
  ;[1 1 1] Spawn the player and put it's hat
  (set `/Game/Blueprints/Main/Main_Pawn.Name` Name (cast `/Game/Blueprints/Main/Main_Pawn` (`Controller.K2_GetPawn` Player) :!pure true))
  (`self.Reposition All Players`))

(event `self.K2_OnLogout`
  (params (ExitingController :type "Controller Object Reference"))
  ;[1 1 1] Event on Logout - Destoy session caller in Game Info Instance
  (bind _asmain_player_controller (cast `/Game/Blueprints/Main/Main_PlayerController` ExitingController))
  (`/Game/Blueprints/WizardGameInstance.Destroy Session Caller` (cast `/Game/Blueprints/WizardGameInstance` (`GameplayStatics.GetGameInstance`) :!pure true) _asmain_player_controller))

(event `Reposition All Players`
  (bind _playercontrollers (`self.PlayerControllers`))
  ;[1 1 1] Position players equaly around the table
  (for (_array_element _array_index) _playercontrollers
    (bind _returnvalue (* _array_index (/ -360.0 (`KismetMathLibrary.Conv_IntToDouble` (`KismetArrayLibrary.Array_Length` _playercontrollers)))))
    (`self.K2_SetActorTransform` (`Controller.K2_GetPawn` _array_element) (`KismetMathLibrary.MakeTransform` (`KismetMathLibrary.MakeVector` (* 100 (`KismetMathLibrary.DegSin` _returnvalue)) (* 100 (`KismetMathLibrary.DegCos` _returnvalue))) (`KismetMathLibrary.MakeRotator` 0.0 0.0 (- (* -1 _returnvalue) 90.0))) false false)))

(event `CheckStartingContition`
  ;[1 1 1] Check if the game is ready to start, then starts the game
  (if (and (not (`self.GameStarted`)) (== (`KismetArrayLibrary.Array_Length` (`self.PlayerControllers`)) (`self.Max Players`)))
    (set `self.GameStarted` true)
    (`KismetSystemLibrary.K2_SetTimerDelegate` (delegate `Start Game`) 2.0)))

(event `Start Game`
  (bind _playercontrollers (`self.PlayerControllers`))
  ;[1 1 1] Check if the game is ready to start, then starts the game
  (bind _asmain_game_state (cast `/Game/Blueprints/Main/Main_GameState` (`GameplayStatics.GetGameState`)))
  (`/Game/Blueprints/Main/Main_GameState.Start Game` _asmain_game_state (`self.PlayerControllers`))
  (for _array_element _playercontrollers
    (for (_array_element_2 _array_index) _playercontrollers
      (if (!= _array_element_2 _array_element)
        (`/Game/Blueprints/Main/Main_PlayerController.IdentifyPlayer` _array_element _array_index (cast `/Game/Blueprints/Main/Main_Pawn` (`Controller.K2_GetPawn` _array_element_2) :!pure true))))))

(fn `UserConstructionScript`)