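; Lobby player state that maps a player's HatID to a hat image from the Hats array.
; When destroyed, it refreshes the player list in the LobbyMenu of player controller 0.
; The Name OnRep is empty, with disconnected logic that would refresh that list and the visible GameSettings players window.
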(event `self.ReceiveTick`
  (params (DeltaSeconds :type "Float (single-precision)")))

(event `self.ReceiveDestroyed`
  (bind _aslobby_player_controller (cast `/Game/Blueprints/Lobby/Lobby_PlayerController` (`GameplayStatics.GetPlayerController` 0)))
  (bind _lobby_menu (`/Game/Blueprints/Lobby/Lobby_PlayerController.Lobby Menu` _aslobby_player_controller))
  (`/Engine/EditorBlueprintResources/StandardMacros.IsValid` _lobby_menu
    (:`Is Valid`
      (`/Game/GUI/Lobby/LobbyMenu.RefreshPlayerList` _lobby_menu))))

(fn `GetHatImage`
  (returns (HatImage :type "Texture2D Object Reference"))
  (return (`|GetArrayItem` (`self.Hats`) (`self.HatID`))))

(fn `OnRep_Name`)

(fn `UserConstructionScript`)